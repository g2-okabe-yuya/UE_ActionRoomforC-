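; BP_MovementFloor is a floor actor in the ActionRoom that moves up and down continuously.
; Tick offsets it one unit per frame along local Z in the direction given by MoveState, without sweep, so its speed depends on frame rate.
; From BeginPlay, a looping chain of delays flips MoveState between up and down every five seconds.
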(event `self.ReceiveBeginPlay`
  (`KismetSystemLibrary.Delay` 3.0 :!label _label)
  (switch `/Game/ActionRoom/Enum/EMovementFloorState` (`self.MoveState`)
    (:`NewEnumerator1`
      (`KismetSystemLibrary.Delay` 2.0)
      (set `self.MoveState` "NewEnumerator2")
      (goto _label))
    (:`NewEnumerator2`
      (`KismetSystemLibrary.Delay` 2.0)
      (set `self.MoveState` "NewEnumerator1")
      (goto _label))))

(event `self.ReceiveTick`
  (params (DeltaSeconds :type "Float (single-precision)"))
  ;[1 1 1] 床の上下移動処理
  (switch `/Game/ActionRoom/Enum/EMovementFloorState` (`self.MoveState`)
    (:`NewEnumerator1`
      (`self.K2_AddActorLocalOffset` (0.0 0.0 1.0)))
    (:`NewEnumerator2`
      (`self.K2_AddActorLocalOffset` (0.0 0.0 -1.0)))))

(fn `UserConstructionScript`)