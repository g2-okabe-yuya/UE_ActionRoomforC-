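; BP_FollowLight is an ActionRoom actor, named as a follow light, that stays positioned above the player character.
; Each Tick it sets its location to the player's location plus a fixed vertical offset, without sweeping.
; A GetPlayer helper caches player character 0 and fetches it again whenever the cached reference is invalid.
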(event `self.ReceiveTick`
  (params (DeltaSeconds :type "Float (single-precision)"))
  (bind _newparam (`self.GetPlayer`))
  ;[1 1 1] Playerに追従する処理
  (`/Engine/EditorBlueprintResources/StandardMacros.IsValid` _newparam
    (:`Is Valid`
      (`self.K2_SetActorLocation` (+ (`self.K2_GetActorLocation` _newparam) (0.0 0.0 150.0))))))

(fn `GetPlayer`
  (returns (NewParam :type "Character Object Reference"))
  ;[1 1 1] Playerを取得
  (`self.Player`
    (:`then`
      _)
    (:`else`
      (set `self.Player` (`GameplayStatics.GetPlayerCharacter` 0))))
  (return (`self.Player`)))

(fn `UserConstructionScript`)